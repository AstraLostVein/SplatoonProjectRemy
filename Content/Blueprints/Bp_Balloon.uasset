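; Destructible balloon target that loses Hp on any damage and is destroyed at zero, with a randomly chosen material from two options.
; Each balloon increments the player BP_Inkling's CountBalloon on BeginPlay and decrements it on EndPlay.
; When the count hits zero and the game sound reference is valid, it stops that sound, disables player input, shows the cursor and opens the win screen.
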(event `self.ReceiveBeginPlay`
  (bind _asbp_inkling (cast `/Game/Blueprints/BP_Inkling` (`GameplayStatics.GetPlayerCharacter` 0)))
  (bind _output_get (set `self.As BP Third Person Character` _asbp_inkling))
  (bind _result (`/Engine/EditorBlueprintResources/StandardMacros.IncrementInt` (`/Game/Blueprints/BP_Inkling.CountBalloon` _output_get))
    (:`  `
      (set `/Game/Blueprints/BP_Inkling.CountBalloon` _result _output_get))))

(event `self.ReceiveAnyDamage`
  (params (Damage :type "Float (single-precision)") (DamageType :type "DamageType Object Reference") (InstigatedBy :type "Controller Object Reference") (DamageCauser :type "Actor Object Reference"))
  (bind _hp (`self.Hp`))
  (set `self.Hp` (- _hp Damage))
  (if (<= _hp 0.0)
    (`self.K2_DestroyActor`)))

(event `self.ReceiveEndPlay`
  (params (EndPlayReason :type "EEndPlayReason Enum" :default "Destroyed"))
  (bind _returnvalue (`GameplayStatics.GetPlayerController` 0))
  (bind _as_bp_third_person_character (`self.As BP Third Person Character`))
  (bind _countballoon (`/Game/Blueprints/BP_Inkling.CountBalloon` _as_bp_third_person_character))
  (bind _result (`/Engine/EditorBlueprintResources/StandardMacros.DecrementInt` _countballoon)
    (:`  `
      (set `/Game/Blueprints/BP_Inkling.CountBalloon` _result _as_bp_third_person_character)
      (if (== _countballoon 0)
        ;[1 1 1] Endgame
        (bind _refsoundgame (`/Game/Blueprints/BP_Inkling.RefSoundGame` _as_bp_third_person_character)
          (:`then`
            (`AudioComponent.Stop` _refsoundgame)
            (`self.DisableInput` _as_bp_third_person_character _returnvalue)
            (set `PlayerController.bShowMouseCursor` true _returnvalue)
            (bind _returnvalue_2 (`|CreateWidget` "/Game/Widget/WBP_WinScreen.WBP_WinScreen_C"))
            (`UserWidget.AddToViewport` _returnvalue_2 0))
          (:`else`))))))

(fn `UserConstructionScript`
  (`PrimitiveComponent.SetMaterial` (`self.Balloon`) 0 (select `int` (`KismetMathLibrary.RandomIntegerInRange` 0 1) :`0` "/Game/AssetSplatoon/balloon/textures/M_Balloon.M_Balloon" :`1` "/Game/AssetSplatoon/balloon/textures/M_Balloon1.M_Balloon1" :!type "MaterialInterface Object Reference")))