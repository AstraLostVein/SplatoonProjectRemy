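; Ink projectile that splats a decal and deals a small amount of damage when its static mesh hits something.
; On hit it attaches a randomly sized, randomly pitched ink decal to the struck component, oriented from the hit location vector.
; It then damages the hit actor, spawns a Bp_BoxDetectInk at the impact point and destroys itself.
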(event `self.StaticMesh.OnComponentHit`
  (params (HitComponent :type "PrimitiveComponent Object Reference") (OtherActor :type "Actor Object Reference") (OtherComp :type "PrimitiveComponent Object Reference") (NormalImpulse :type "Vector Structure") (Hit :type "HitResult Structure (by ref)"))
  (bind _returnvalue (`KismetMathLibrary.RandomFloatInRange` 50.0 100.0))
  (bind _returnvalue_2 (`KismetMathLibrary.MakeRotFromX` Hit_Location))
  (bind _returnvalue_3 (`GameplayStatics.SpawnDecalAttached` "/Game/MatInk/M_Ink.M_Ink" (`KismetMathLibrary.MakeVector` _returnvalue _returnvalue _returnvalue) OtherComp "None" (`self.K2_GetActorLocation`) _returnvalue_2 "KeepWorldPosition"))
  (`SceneComponent.K2_AddRelativeRotation` _returnvalue_3 (`KismetMathLibrary.MakeRotator` 0.0 (`KismetMathLibrary.RandomFloatInRange` 0.0 360.0)) false false)
  (`GameplayStatics.ApplyDamage` Hit_HitActor 5.0)
  (`|SpawnActorFromClass` "/Game/Blueprints/Bp_BoxDetectInk.Bp_BoxDetectInk_C" (`KismetMathLibrary.MakeTransform` Hit_Location _returnvalue_2 (1.5 1.5 1.5)) "AlwaysSpawn" "MultiplyWithRoot" null null)
  (`self.K2_DestroyActor`))

(fn `UserConstructionScript`)